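; Shooter HUD that draws a dynamic four-piece crosshair at the center of the screen.
; Each DrawHUD pass reads the spread multiplier from BP_ShooterCharacter and scales it by CrossHairSpreadMax to push the top, bottom, left and right textures outward.
; The character reference is cached from player pawn 0 on BeginPlay and re-acquired during drawing whenever it is invalid.
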(event EventBeginPlay
  (Utilities|IsValid (Variables|Default|GetShooterCharacter)
    (:Is%20Not%20Valid
      (bind _asbp_shooter_character (Utilities|Casting|CastToBP_ShooterCharacter (Game|Player|GetPlayerPawn 0)))
      (Variables|Default|SetShooterCharacter _asbp_shooter_character))))

(event EventDrawHUD
  (params (SizeX :type Integer) (SizeY :type Integer))
  (Variables|Default|SetScreen%20Center (Math|Vector2D|MakeVector2D (Math|Conversions|ToFloat(Integer) (/ SizeX 2)) (Math|Conversions|ToFloat(Integer) (/ SizeY 2))))
  (Utilities|IsValid (Variables|Default|GetShooterCharacter)
    (:Is%20Valid
      _)
    (:Is%20Not%20Valid
      (bind _asbp_shooter_character (Utilities|Casting|CastToBP_ShooterCharacter (Game|Player|GetPlayerPawn 0)))
      (Variables|Default|SetShooterCharacter _asbp_shooter_character)))
  (Variables|Default|SetCrossHairSpreadMultiplier (Class|ShooterCharacter|GetCrossHairSpreadMultiplier (Variables|Default|GetShooterCharacter)))
  (Variables|Default|SetCrossHairBaseCenter (Math|Vector2D|MakeVector2D (- (.X (Math|Vector2D|BreakVector2D (Variables|Default|GetScreen%20Center))) 32.0) (- (.Y (Math|Vector2D|BreakVector2D (Variables|Default|GetScreen%20Center))) 32.0)))
  (Canvas|DrawTexture "/Game/_Game/Assets/Textures/CrossHairs/Quad_9_Bottom.Quad_9_Bottom" (.X (Math|Vector2D|BreakVector2D (Variables|Default|GetCrossHairBaseCenter))) (+ (.Y (Math|Vector2D|BreakVector2D (Variables|Default|GetCrossHairBaseCenter))) (* (Variables|Default|GetCrossHairSpreadMax) (Variables|Default|GetCrossHairSpreadMultiplier))) 64.0 64.0 0.0 0.0 1.0 1.0 "(R=1.000000,G=1.000000,B=1.000000,A=1.000000)")
  (Canvas|DrawTexture "/Game/_Game/Assets/Textures/CrossHairs/Quad_9_Top.Quad_9_Top" (.X (Math|Vector2D|BreakVector2D (Variables|Default|GetCrossHairBaseCenter))) (- (.Y (Math|Vector2D|BreakVector2D (Variables|Default|GetCrossHairBaseCenter))) (* (Variables|Default|GetCrossHairSpreadMultiplier) (Variables|Default|GetCrossHairSpreadMax))) 64.0 64.0 0.0 0.0 1.0 1.0 "(R=1.000000,G=1.000000,B=1.000000,A=1.000000)")
  (Canvas|DrawTexture "/Game/_Game/Assets/Textures/CrossHairs/Quad_9_Left.Quad_9_Left" (- (.X (Math|Vector2D|BreakVector2D (Variables|Default|GetCrossHairBaseCenter))) (* (Variables|Default|GetCrossHairSpreadMultiplier) (Variables|Default|GetCrossHairSpreadMax))) (.Y (Math|Vector2D|BreakVector2D (Variables|Default|GetCrossHairBaseCenter))) 64.0 64.0 0.0 0.0 1.0 1.0 "(R=1.000000,G=1.000000,B=1.000000,A=1.000000)")
  (Canvas|DrawTexture "/Game/_Game/Assets/Textures/CrossHairs/Quad_9_Right.Quad_9_Right" (+ (.X (Math|Vector2D|BreakVector2D (Variables|Default|GetCrossHairBaseCenter))) (* (Variables|Default|GetCrossHairSpreadMultiplier) (Variables|Default|GetCrossHairSpreadMax))) (.Y (Math|Vector2D|BreakVector2D (Variables|Default|GetCrossHairBaseCenter))) 64.0 64.0 0.0 0.0 1.0 1.0 "(R=1.000000,G=1.000000,B=1.000000,A=1.000000)"))

(fn ConstructionScript)