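; BP_Truck is a factory truck actor that plays a crash test with a cockpit and dummy.
; StartTruck rewinds both skeletal animations, then a timeline slides the cockpit along X.
; When the move ends, a crash sound plays and both animations run.
; A polling loop waits for the dummy animation to finish, then resets the DoOnce after a short delay so it can run again.
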(event Custom|StartTruck
  (bind _sk_truck_sm_dummy (Variables|Default|GetSK_Truck_SM_Dummy))
  (Utilities|FlowControl|DoOnce false :!label _label
    (:Completed
      (Components|Animation|SetPosition (Variables|Default|GetSK_Truck_SM_Truck_Cockpit) 0.0 false)
      (bind _move (Timeline|Move PlayFromStart)
        (:Update
          (Transformation|SetRelativeLocation (Variables|Default|GetSK_Truck_SM_Truck_Cockpit) (Math|Vector|MakeVector _move 0.0 0.0) false false))
        (:Finished
          (Audio|PlaySoundatLocation "/Game/Audio/S_Car_crash.S_Car_crash" (Transformation|GetActorLocation) "0, 0, 0" 3.0 1.0 0.0 0 0 0)
          (Components|Animation|SetPosition _sk_truck_sm_dummy 0.05 true)
          (Audio|Components|Audio|Play _sk_truck_sm_dummy false)
          (if (Audio|Components|Audio|IsPlaying _sk_truck_sm_dummy) :!label _label_2
            (Utilities|FlowControl|Delay 0.2)
            (goto _label_2)
            (else
              (Utilities|FlowControl|Delay 2.0)
              (goto _label Reset))))))))

(fn ConstructionScript)